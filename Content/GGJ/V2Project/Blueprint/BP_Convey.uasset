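; BP_Convey is a conveyor actor that passes resources along through its Finish event.
; The construction script runs the parent's logic, then sets the SplineMesh start to the actor's world location and its end to a fixed X offset from that.
; Finish tells the incoming Ressource to RSMoveTo this conveyor, while BeginPlay only calls the parent.
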(event `self.ReceiveBeginPlay`
  (`parent.ReceiveBeginPlay`))

(event `/Game/GGJ/V2Project/Blueprint/BPI_Engine.Finish`
  (params (Ressource :type "/Game/GGJ/V2Project/Blueprint/BP_Ressource Object Reference"))
  (`/Game/GGJ/V2Project/Blueprint/BP_Ressource.RS_MoveTo` Ressource self))

(fn `UserConstructionScript`
  (`parent.UserConstructionScript`)
  (`SplineMeshComponent.SetStartPosition` (`self.SplineMesh`) (`self.K2_GetActorLocation`) true)
  (`SplineMeshComponent.SetEndPosition` (`self.SplineMesh`) (+ (`self.K2_GetActorLocation`) (600.0 0.0 0.0)) true))