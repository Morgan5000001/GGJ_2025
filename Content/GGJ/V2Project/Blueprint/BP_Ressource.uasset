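; BP_Ressource is a resource actor whose mesh can be switched to an iron bar look.
; On BeginPlay it gives the mesh a dynamic instance of M_Basic.
; Apply detaches the actor in world space and calls MC_SetMaterial, which swaps that instance's texture to T_IronBar.
; A separate RS_DisablePhysics event turns off the mesh's physics simulation and collision.
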(event `self.ReceiveBeginPlay`
  (bind _returnvalue (`KismetMaterialLibrary.CreateDynamicMaterialInstance` "/Game/GGJ/V2Project/M_Basic.M_Basic"))
  (bind _output_get (set `self.Material` _returnvalue))
  (`PrimitiveComponent.SetMaterial` (`self.RessourceMesh`) 0 _output_get))

(event `MC_SetMaterial`
  (`MaterialInstanceDynamic.SetTextureParameterValue` (`self.Material`) "Texture" "/Game/GGJ/V2Project/T_IronBar.T_IronBar"))

(event `/Game/GGJ/V2Project/Blueprint/BPI_Engine.Apply`
  (params (InitEngine :type "/Game/GGJ/V2Project/Blueprint/BP_ModuleParent Object Reference"))
  (`self.K2_DetachFromActor` "KeepWorld" "KeepWorld" "KeepWorld")
  (`self.MC_SetMaterial`))

(event `RS_DisablePhysics`
  (`PrimitiveComponent.SetSimulatePhysics` (`self.RessourceMesh`) false)
  (`PrimitiveComponent.SetCollisionEnabled` (`self.RessourceMesh`) "NoCollision"))

(fn `UserConstructionScript`)