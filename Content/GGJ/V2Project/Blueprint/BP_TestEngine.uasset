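; Test crafting engine that turns BP_Ressource actors into recipe outputs and hands them to a linked OutModule.
; Resources arriving by box overlap or Finish message attach to the machine, or merge quantity into a matching one.
; A recipe match sets the alarm color and starts a Top animation timeline.
; Its Transformed event consumes inputs and spawns the output, which is forwarded when the timeline finishes.
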(event `RS_Finished`
  (`/Engine/EditorBlueprintResources/StandardMacros.IsValid` (`self.OutModule`)
    (:`Is Valid`
      (message `/Game/GGJ/V2Project/Blueprint/BPI_Engine.Finish` (`self.OutModule`) (`self.OutputRessource`))
      (`KismetArrayLibrary.Array_RemoveItem` (`self.Ressources`) (`self.OutputRessource`))
      (set `self.OutputRessource` null))))

(event `RS_StartEngine`
  ;[1 1 1] Animation
  (bind (_direction _alpha) (`Timeline|Timeline` :!via `PlayFromStart`)
    (:`Update`
      (`SceneComponent.K2_SetRelativeLocation` (`self.Top`) (`KismetMathLibrary.VLerp` (0.0 0.0 200.0) (0.0 0.0 100.0) _alpha) false false))
    (:`Finished`
      (`self.RS_Finished`))
    (:`Transformed`
      (`self.RS_EngineApply`))))

(event `self.ReceiveBeginPlay`
  (`parent.ReceiveBeginPlay`))

(event `/Game/GGJ/V2Project/Blueprint/BPI_Engine.Interact`
  (params (Investigator :type "Actor Object Reference")))

(event `RS_EngineApply`
  (`self.DestroyOtherRessources`))

(event `MC_SetAlarmColor`
  (params (`Work?` :type Boolean))
  ;[0 0 0] Feedback alarme à refaire
  (`MaterialInstanceDynamic.SetVectorParameterValue` (`self.Material`) "BaseColor" (select `bool` `Work?` :`false` (struct :`R` 0.694118 :`A` 1.0) :`true` (struct :`R` 0.023906 :`G` 1.0 :`B` 0.00239 :`A` 1.0) :!type "LinearColor Structure")))

(event `RS_AttachRessource`
  (params (Ressource :type "/Game/GGJ/V2Project/Blueprint/BP_Ressource Object Reference"))
  (`self.K2_AttachToComponent` Ressource (`self.AttachedScene`) "None" "SnapToTarget" "SnapToTarget" "KeepRelative" true))

(event `self.Box.OnComponentBeginOverlap`
  (params (OverlappedComponent :type "PrimitiveComponent Object Reference") (OtherActor :type "Actor Object Reference") (OtherComp :type "PrimitiveComponent Object Reference") (OtherBodyIndex :type Integer) (bFromSweep :type Boolean) (SweepResult :type "HitResult Structure (by ref)"))
  ;[1 1 1] OverlapDetection
  (bind _asbp_ressource (cast `/Game/GGJ/V2Project/Blueprint/BP_Ressource` OtherActor))
  (`self.RS_OverlapDetected` _asbp_ressource))

(event `RS_OverlapDetected`
  (params (RessourceDetected :type "/Game/GGJ/V2Project/Blueprint/BP_Ressource Object Reference"))
  (bind (_ressource_resource _ressource_quantity) (break `Ressource` (`/Game/GGJ/V2Project/Blueprint/BP_Ressource.GetRessource` RessourceDetected)))
  ;[1 1 1] OverlapDetection
  (bind (_isfind _ressourcefinded) (`self.Find Ressource` RessourceDetected))
  (if (not _isfind)
    (`KismetArrayLibrary.Array_Add` (`self.Ressources`) RessourceDetected)
    (`/Game/GGJ/V2Project/Blueprint/BP_Ressource.RS_DisablePhysics` RessourceDetected)
    (`self.RS_AttachRessource` RessourceDetected)
    (bind (_recipefind _receipefinded) (`self.Find Recipe`))
    (`self.MC_SetAlarmColor` _recipefind) ; Feedback alarme mais à refaire
    (if _recipefind
      (set `self.CurrentReceipe` _receipefinded)
      (`self.RS_StartEngine`) ; Voir si besoin d'énergie ou pas
    )
    (else
      (`/Game/GGJ/V2Project/Blueprint/BP_Ressource.RS_AddToQuantity` _ressourcefinded _ressource_quantity)
      (`self.K2_DestroyActor` RessourceDetected))))

(event `/Game/GGJ/V2Project/Blueprint/BPI_Engine.Finish`
  (params (Ressource :type "/Game/GGJ/V2Project/Blueprint/BP_Ressource Object Reference"))
  (`self.RS_OverlapDetected` Ressource))

(event `RS_MoveToPosition`
  (params (Ressource :type "/Game/GGJ/V2Project/Blueprint/BP_Ressource Object Reference"))
  (`KismetArrayLibrary.Array_Add` (`self.Ressources`) Ressource)
  (`self.RS_AttachRessource` Ressource))

(fn `DestroyOtherRessources`
  (locals (AllRessources :type "Array of /Game/GGJ/V2Project/Blueprint/BP_Ressource Object Reference"))
  (set `local.AllRessources` (`self.Ressources`))
  (for _array_element (`local.AllRessources`)
    (if (`KismetArrayLibrary.Array_Contains` (`RecipeDataAsset.GetInputs` (`self.CurrentReceipe`)) (`/Game/GGJ/V2Project/Blueprint/BP_Ressource.GetRessource` _array_element))
      (bind _shoulddestroyactor (`/Game/GGJ/V2Project/Blueprint/BP_Ressource.RemoveQuantity` _array_element 1))
      (if _shoulddestroyactor
        (`KismetArrayLibrary.Array_RemoveItem` (`self.Ressources`) _array_element)
        (`self.K2_DestroyActor` _array_element))))
  (bind _returnvalue (`|SpawnActorFromClass` "/Game/GGJ/V2Project/Blueprint/BP_Ressource.BP_Ressource_C" (`SceneComponent.K2_GetComponentToWorld` (`self.AttachedScene`)) "Undefined" "MultiplyWithRoot" null (`RecipeDataAsset.GetRessourceOut` (`self.CurrentReceipe`)) null))
  (set `self.OutputRessource` _returnvalue))

(fn `Find Recipe`
  (returns (RecipeFind :type Boolean) (ReceipeFinded :type "RecipeDataAsset Object Reference"))
  (locals (CanDoReceipe :type Boolean :default false))
  (for _array_element (`self.Receipe`)
    (if (`RecipeDataAsset.CanCraft` _array_element (`self.ReturnArrayRessources`))
      (return true _array_element)))
  (return false null))

(fn `Find Ressource`
  (params (RessourceDetected :type "/Game/GGJ/V2Project/Blueprint/BP_Ressource Object Reference"))
  (returns (IsFind :type Boolean) (RessourceFinded :type "/Game/GGJ/V2Project/Blueprint/BP_Ressource Object Reference"))
  (for _array_element (`self.Ressources`)
    (if (== (`/Game/GGJ/V2Project/Blueprint/BP_Ressource.GetRessourceData` _array_element) (`/Game/GGJ/V2Project/Blueprint/BP_Ressource.GetRessourceData` (`local.RessourceDetected`)))
      (return true _array_element)))
  (return false null))

(fn `ReturnArrayRessources`
  (returns (Ressources :type "Map of RessourceDataAsset Object Reference to Integer"))
  (locals (NewLocalVar :type "Map of RessourceDataAsset Object Reference to Object Object Reference"))
  (for _array_element (`self.Ressources`)
    (bind (_ressource_resource _ressource_quantity) (break `Ressource` (`/Game/GGJ/V2Project/Blueprint/BP_Ressource.GetRessource` _array_element)))
    (`BlueprintMapLibrary.Map_Add` (`local.NewLocalVar`) _ressource_resource _ressource_quantity))
  (return (`local.NewLocalVar`)))

(fn `UserConstructionScript`
  (`parent.UserConstructionScript`))