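; BP_EngineParent is a base actor, named as the parent for engines, whose visual mesh is driven by build data.
; On BeginPlay it passes its own BuildData to RefreshBuild.
; RefreshBuild stores the supplied build and sets the StaticMesh component to the mesh returned by that build's GetMesh, so the same event can swap builds.
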(event `self.ReceiveBeginPlay`
  (`parent.ReceiveBeginPlay`)
  (`self.RefreshBuild` (`self.BuildData`)))

(event `RefreshBuild`
  (params (Build :type "BuildableDataAsset Object Reference"))
  (bind _output_get (set `self.BuildData` Build))
  (`StaticMeshComponent.SetStaticMesh` (`self.StaticMesh`) (`BuildableDataAsset.GetMesh` _output_get)))

(fn `UserConstructionScript`
  (`parent.UserConstructionScript`))