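; Custom game instance that owns the game's save object and handles accepted session invites.
; It creates or loads a BP_CustomSave, then writes it to one slot whenever inventory, gold or placed machine locations change through its save events.
; Inventory and gold are read from the first-person character, ignoring the passed-in values.
; Accepting an invite ends and destroys the current session, then joins the new one even if either step fails.
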(event `LoadSave`
  (bind _returnvalue (`GameplayStatics.LoadGameFromSlot` "SaveInventory"))
  (bind _asbp_custom_save (cast `/Game/GGJ/Blueprint/BP_CustomSave` _returnvalue))
  (set `self.SaveRef` _asbp_custom_save))

(event `InitSave`
  (bind _returnvalue (`GameplayStatics.CreateSaveGameObject` "/Game/GGJ/Blueprint/BP_CustomSave.BP_CustomSave_C"))
  (set `self.SaveRef` _returnvalue))

(event `SaveInventory`
  (params (`Inventory To Save` :type "Array of /Game/GGJ/Blueprint/Inventory/S_Item Structure"))
  (set `/Game/GGJ/Blueprint/BP_CustomSave.Inventory` (`/Game/GGJ/Blueprint/Inventory/BP_Inventory.Inventory` (`/Game/GGJ/Blueprint/FirstPerson/Blueprints/BP_FirstPersonCharacter.BP_Inventory` (cast `/Game/GGJ/Blueprint/FirstPerson/Blueprints/BP_FirstPersonCharacter` (`GameplayStatics.GetPlayerCharacter` 0) :!pure true))) (`self.SaveRef`))
  (`GameplayStatics.SaveGameToSlot` (`self.SaveRef`) "SaveInventory"))

(event `SaveBatAdd`
  (params (Machine :type "/Game/GGJ/Blueprint/Machines/BP_ParentMachines Class Reference") (Tranform :type "Transform Structure"))
  (`BlueprintMapLibrary.Map_Add` (`/Game/GGJ/Blueprint/BP_CustomSave.MachinesLocations` (`self.SaveRef`)) Tranform Machine)
  (`GameplayStatics.SaveGameToSlot` (`self.SaveRef`) "SaveInventory"))

(event `SaveBatRemove`
  (params (Key :type "Transform Structure (by ref)"))
  (`BlueprintMapLibrary.Map_Remove` (`/Game/GGJ/Blueprint/BP_CustomSave.MachinesLocations` (`self.SaveRef`)) Key)
  (`GameplayStatics.SaveGameToSlot` (`self.SaveRef`) "SaveInventory"))

(event `SaveGold`
  (params (Gold :type "Float (double-precision)"))
  (set `/Game/GGJ/Blueprint/BP_CustomSave.Gold` (`/Game/GGJ/Blueprint/FirstPerson/Blueprints/BP_FirstPersonCharacter.Gold` (cast `/Game/GGJ/Blueprint/FirstPerson/Blueprints/BP_FirstPersonCharacter` (`GameplayStatics.GetPlayerCharacter` 0) :!pure true)) (`self.SaveRef`))
  (`GameplayStatics.SaveGameToSlot` (`self.SaveRef`) "SaveInventory"))

(event `self.OnSessionInviteAccepted`
  (params (LocalPlayerNum :type Integer) (PersonInvited :type "BPUniqueNetId Structure") (SessionToJoin :type "BlueprintSessionResult Structure (by ref)"))
  (bind _returnvalue (`GameplayStatics.GetPlayerController` 0))
  (`EndSessionCallbackProxy.EndSession` _returnvalue
    (:`OnSuccess`
      _)
    (:`OnFailure`
      _))
  (`DestroySessionCallbackProxy.DestroySession` _returnvalue
    (:`OnSuccess`
      _)
    (:`OnFailure`
      _))
  (`JoinSessionCallbackProxy.JoinSession` _returnvalue SessionToJoin))