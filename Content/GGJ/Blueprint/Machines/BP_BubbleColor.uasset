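; Bubble-coloring machine that outputs bubble items of the current shape and selected color into its result inventory.
; A one-second poll waits for the start condition, then, if bubbles are present, starts a looping production timer.
; Each tick switches on shape and color to add one matching item, with Level scaling speed and capacity.
; Interacting outside build mode advances the color and machine material, provided no shaped bubbles are held.
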(event `SendRondNormal`
  ;[1 0.5842 0] Send bubbles
  (bind _return_inventory (`/Game/GGJ/Blueprint/Inventory/BFL_InventoryGestion.AddItemInventory` (make `/Game/GGJ/Blueprint/Inventory/S_Item` "NewEnumerator1" "NewEnumerator1" 0 "/Game/GGJ/Image/Bubbles/Round/MI_RoundNormalBubble.MI_RoundNormalBubble") 1 (`self.ResultInventoryMachin`) (* (`self.QuantityMaxDefault`) (`self.Level`))))
  (set `self.ResultInventoryMachin` _return_inventory))

(event `SendCarréNormal`
  ;[1 0.5842 0] Send bubbles
  (bind _return_inventory (`/Game/GGJ/Blueprint/Inventory/BFL_InventoryGestion.AddItemInventory` (make `/Game/GGJ/Blueprint/Inventory/S_Item` "NewEnumerator2" "NewEnumerator1" 0 "/Game/GGJ/Image/Bubbles/Square/MI_SquareNormalBubble.MI_SquareNormalBubble") 1 (`self.ResultInventoryMachin`) (* (`self.QuantityMaxDefault`) (`self.Level`))))
  (set `self.ResultInventoryMachin` _return_inventory))

(event `SendTriangleNormal`
  ;[1 0.5842 0] Send bubbles
  (bind _return_inventory (`/Game/GGJ/Blueprint/Inventory/BFL_InventoryGestion.AddItemInventory` (make `/Game/GGJ/Blueprint/Inventory/S_Item` "NewEnumerator3" "NewEnumerator1" 0 "/Game/GGJ/Image/Bubbles/Triangle/MI_TriangleNormalBubble.MI_TriangleNormalBubble") 1 (`self.ResultInventoryMachin`) (* (`self.QuantityMaxDefault`) (`self.Level`))))
  (set `self.ResultInventoryMachin` _return_inventory))

(event `SendRondBleu`
  ;[1 0.5842 0] Send bubbles
  (bind _return_inventory (`/Game/GGJ/Blueprint/Inventory/BFL_InventoryGestion.AddItemInventory` (make `/Game/GGJ/Blueprint/Inventory/S_Item` "NewEnumerator1" "NewEnumerator2" 0 "/Game/GGJ/Image/Bubbles/Round/MI_RoundBlueBubble.MI_RoundBlueBubble") 1 (`self.ResultInventoryMachin`) (* (`self.QuantityMaxDefault`) (`self.Level`))))
  (set `self.ResultInventoryMachin` _return_inventory))

(event `SendCarréBleu`
  ;[1 0.5842 0] Send bubbles
  (bind _return_inventory (`/Game/GGJ/Blueprint/Inventory/BFL_InventoryGestion.AddItemInventory` (make `/Game/GGJ/Blueprint/Inventory/S_Item` "NewEnumerator2" "NewEnumerator2" 0 "/Game/GGJ/Image/Bubbles/Square/MI_SquareBlueBubble.MI_SquareBlueBubble") 1 (`self.ResultInventoryMachin`) (* (`self.QuantityMaxDefault`) (`self.Level`))))
  (set `self.ResultInventoryMachin` _return_inventory))

(event `SendTriangleBleu`
  ;[1 0.5842 0] Send bubbles
  (bind _return_inventory (`/Game/GGJ/Blueprint/Inventory/BFL_InventoryGestion.AddItemInventory` (make `/Game/GGJ/Blueprint/Inventory/S_Item` "NewEnumerator3" "NewEnumerator2" 0 "/Game/GGJ/Image/Bubbles/Triangle/MI_TriangleBlueBubble.MI_TriangleBlueBubble") 1 (`self.ResultInventoryMachin`) (* (`self.QuantityMaxDefault`) (`self.Level`))))
  (set `self.ResultInventoryMachin` _return_inventory))

(event `SendRondRouge`
  ;[1 0.5842 0] Send bubbles
  (bind _return_inventory (`/Game/GGJ/Blueprint/Inventory/BFL_InventoryGestion.AddItemInventory` (make `/Game/GGJ/Blueprint/Inventory/S_Item` "NewEnumerator1" "NewEnumerator3" 0 "/Game/GGJ/Image/Bubbles/Round/MI_RoundRedBubble.MI_RoundRedBubble") 1 (`self.ResultInventoryMachin`) (* (`self.QuantityMaxDefault`) (`self.Level`))))
  (set `self.ResultInventoryMachin` _return_inventory))

(event `SendCarréRouge`
  ;[1 0.5842 0] Send bubbles
  (bind _return_inventory (`/Game/GGJ/Blueprint/Inventory/BFL_InventoryGestion.AddItemInventory` (make `/Game/GGJ/Blueprint/Inventory/S_Item` "NewEnumerator2" "NewEnumerator3" 0 "/Game/GGJ/Image/Bubbles/Square/MI_SquareRedBubble.MI_SquareRedBubble") 1 (`self.ResultInventoryMachin`) (* (`self.QuantityMaxDefault`) (`self.Level`))))
  (set `self.ResultInventoryMachin` _return_inventory))

(event `SendTriangleRouge`
  ;[1 0.5842 0] Send bubbles
  (bind _return_inventory (`/Game/GGJ/Blueprint/Inventory/BFL_InventoryGestion.AddItemInventory` (make `/Game/GGJ/Blueprint/Inventory/S_Item` "NewEnumerator3" "NewEnumerator3" 0 "/Game/GGJ/Image/Bubbles/Triangle/MI_TriangleRedBubble.MI_TriangleRedBubble") 1 (`self.ResultInventoryMachin`) (* (`self.QuantityMaxDefault`) (`self.Level`))))
  (set `self.ResultInventoryMachin` _return_inventory))

(event `SendRondVert`
  ;[1 0.5842 0] Send bubbles
  (bind _return_inventory (`/Game/GGJ/Blueprint/Inventory/BFL_InventoryGestion.AddItemInventory` (make `/Game/GGJ/Blueprint/Inventory/S_Item` "NewEnumerator1" "NewEnumerator4" 0 "/Game/GGJ/Image/Bubbles/Round/MI_RoundGreenBubble.MI_RoundGreenBubble") 1 (`self.ResultInventoryMachin`) (* (`self.QuantityMaxDefault`) (`self.Level`))))
  (set `self.ResultInventoryMachin` _return_inventory))

(event `SendCarréVert`
  ;[1 0.5842 0] Send bubbles
  (bind _return_inventory (`/Game/GGJ/Blueprint/Inventory/BFL_InventoryGestion.AddItemInventory` (make `/Game/GGJ/Blueprint/Inventory/S_Item` "NewEnumerator2" "NewEnumerator4" 0 "/Game/GGJ/Image/Bubbles/Square/MI_SquareGreenBubble.MI_SquareGreenBubble") 1 (`self.ResultInventoryMachin`) (* (`self.QuantityMaxDefault`) (`self.Level`))))
  (set `self.ResultInventoryMachin` _return_inventory))

(event `SendTriangleVert`
  ;[1 0.5842 0] Send bubbles
  (bind _return_inventory (`/Game/GGJ/Blueprint/Inventory/BFL_InventoryGestion.AddItemInventory` (make `/Game/GGJ/Blueprint/Inventory/S_Item` "NewEnumerator3" "NewEnumerator4" 0 "/Game/GGJ/Image/Bubbles/Triangle/MI_TriangleGreenBubble.MI_TriangleGreenBubble") 1 (`self.ResultInventoryMachin`) (* (`self.QuantityMaxDefault`) (`self.Level`))))
  (set `self.ResultInventoryMachin` _return_inventory))

(event `StartColoring`
  (bind _bubbles (`self.Bubbles`))
  ;[0 1 0.09229] Je sais plus
  (if (> _bubbles 0)
    (`KismetSystemLibrary.PrintString` (`KismetStringLibrary.Conv_IntToString` _bubbles))
    (bind _returnvalue (`KismetSystemLibrary.K2_SetTimerDelegate` (delegate `Send Bubbles`) (/ (`self.DefaultTime`) (`self.Level`)) true))
    (set `self.TimerProd` _returnvalue)
    (else
      (`KismetSystemLibrary.K2_ClearAndInvalidateTimerHandle` (`self.TimerProd`)))))

(event `Send Bubbles`
  ;[0 1 0.09229] Je sais plus
  (switch `/Game/GGJ/Blueprint/Inventory/E_BulleType` (`self.Shape`)
    (:`NewEnumerator1`
      (switch `/Game/GGJ/Blueprint/Inventory/E_BulleColor` (`self.Colors`)
        (:`NewEnumerator1`
          (`self.SendRondNormal`))
        (:`NewEnumerator2`
          (`self.SendRondBleu`))
        (:`NewEnumerator3`
          (`self.SendRondRouge`))
        (:`NewEnumerator4`
          (`self.SendRondVert`))))
    (:`NewEnumerator2`
      (switch `/Game/GGJ/Blueprint/Inventory/E_BulleColor` (`self.Colors`)
        (:`NewEnumerator1`
          (`self.SendCarréNormal`))
        (:`NewEnumerator2`
          (`self.SendCarréBleu`))
        (:`NewEnumerator3`
          (`self.SendCarréRouge`))
        (:`NewEnumerator4`
          (`self.SendCarréVert`))))
    (:`NewEnumerator3`
      (switch `/Game/GGJ/Blueprint/Inventory/E_BulleColor` (`self.Colors`)
        (:`NewEnumerator1`
          (`self.SendTriangleNormal`))
        (:`NewEnumerator2`
          (`self.SendTriangleBleu`))
        (:`NewEnumerator3`
          (`self.SendTriangleRouge`))
        (:`NewEnumerator4`
          (`self.SendTriangleVert`))))))

(event `self.ReceiveBeginPlay`
  ;[1 0 0.02402] Begin play
  (bind _returnvalue (`KismetSystemLibrary.K2_SetTimerDelegate` (delegate `Is It ok to start?`) 1.0 true))
  (set `self.TimerStart` _returnvalue))

(event `Is It ok to start?`
  ;[1 0 0.02402] Begin play
  (if (`self.IsItOkToStart?`)
    (`KismetSystemLibrary.K2_ClearAndInvalidateTimerHandle` (`self.TimerStart`))
    (`self.StartColoring`)
    (else
      (`KismetSystemLibrary.K2_ClearAndInvalidateTimerHandle` (`self.TimerProd`)))))

(event `/Game/GGJ/Blueprint/Interact/BPI_Interact.Interact`
  (params (PlayerRef :type "/Game/FirstPerson/Blueprints/BP_FirstPersonCharacter Object Reference"))
  ;[0 0.1116 1] Switch shapes
  (if (`/Game/GGJ/Blueprint/BuildMode/BP_BuildComponent.BuildMode ?` (`/Game/FirstPerson/Blueprints/BP_FirstPersonCharacter.BP_BuildComponent` PlayerRef))
    _
    (elif (or (>= (`self.SquareBubbles`) 1) (>= (`self.TriangleBubbles`) 1) (>= (`self.RoundBubbles`) 1))
      _
      (elif (> (`self.Colors`) 4)
        (set `self.Colors` "NewEnumerator0")
        (else
          (bind _output_get (set `self.Colors` (cast `/Game/GGJ/Blueprint/Inventory/E_BulleColor` (+ (`self.Colors`) 1))))
          (`KismetSystemLibrary.PrintString` (`|GetEnumeratorNameAsString` _output_get))
          (`self.UpdateColor`))))))

(event `UpdateColor`
  ;[0 0.1116 1] Switch shapes
  (`PrimitiveComponent.SetMaterial` (`self.Machine`) 0 (select `/Game/GGJ/Blueprint/Inventory/E_BulleColor` (`self.Colors`) :`NewEnumerator1` "/Game/Game_art/asset/lambert2.lambert2" :`NewEnumerator2` "/Game/Game_art/asset/lambert3.lambert3" :`NewEnumerator3` "/Game/GGJ/Mat/M_PreviewWrong.M_PreviewWrong" :`NewEnumerator4` "/Game/GGJ/Mat/M_PreviewTrue.M_PreviewTrue" :!type "MaterialInterface Object Reference")))

(fn `UserConstructionScript`
  (`parent.UserConstructionScript`))