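; BP_Evier is an interactable sink machine where the player produces bubbles.
; Interact toggles crafting: it freezes character movement and turns on the bubble effect, or restores movement and clears both timer and effect.
; While active, a looping timer adds a normal bubble to the player's inventory and spawns a Niagara burst.
; Each interaction also notifies the player's tutorial component, if present; spline interaction always reports no connection.
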(event `self.ReceiveBeginPlay`
  ;[1 1 1] Début du lancement
  ;[1 1 1] Référence au personnage à la premiere personne
  (bind _asbp_first_person_character (cast `/Game/FirstPerson/Blueprints/BP_FirstPersonCharacter` (`GameplayStatics.GetPlayerCharacter` 0)))
  (set `self.As BP First Person Character` _asbp_first_person_character))

(event `/Game/GGJ/Blueprint/Interact/BPI_Interact.Interact`
  (params (PlayerRef :type "/Game/FirstPerson/Blueprints/BP_FirstPersonCharacter Object Reference"))
  (bind _returnvalue (`self.GetComponentByClass` (`self.As BP First Person Character`) "/Game/Blueprints/Tutoriel/BP_Tutoriel.BP_Tutoriel_C"))
  (`|ExecutionSequence`
    (:`then_0`
      (if (`self.CanMakeBubbles?`)
        ;[1 1 1] On ne bouge plus devant l'évier
        (`ActorComponent.Deactivate` (`Character.CharacterMovement` (`self.As BP First Person Character`)))
        (bind _returnvalue_2 (`KismetSystemLibrary.K2_SetTimerDelegate` (delegate `Crafting Bubbles`) 3.0 true))
        (set `self.Timer` _returnvalue_2)
        (set `self.CanMakeBubbles?` false)
        (`ActorComponent.Activate` (`self.NS_Bubbles`) false)
        (else
          (`KismetSystemLibrary.K2_ClearAndInvalidateTimerHandle` (`self.Timer`))
          (`ActorComponent.Activate` (`Character.CharacterMovement` (`self.As BP First Person Character`)) false)
          (set `self.CanMakeBubbles?` true)
          (`ActorComponent.Deactivate` (`self.NS_Bubbles`)))))
    (:`then_1`
      (`/Engine/EditorBlueprintResources/StandardMacros.IsValid` _returnvalue
        (:`Is Valid`
          (message `/Game/Blueprints/Tutoriel/BPi_Tutoriel.InteractEvier` _returnvalue self))))))

(event `Crafting Bubbles`
  (`/Game/GGJ/Blueprint/Inventory/BP_Inventory.AddBubble` (`/Game/FirstPerson/Blueprints/BP_FirstPersonCharacter.BP_Inventory` (stale `/Game/GGJ/Blueprint/Interact/BPI_Interact.Interact` PlayerRef)) (make `/Game/GGJ/Blueprint/Inventory/S_Item` "NewEnumerator1" "NewEnumerator1" 0 "/Game/GGJ/Image/Bubbles/Round/MI_RoundNormalBubble.MI_RoundNormalBubble") 1)
  (`NiagaraFunctionLibrary.SpawnSystemAtLocation` "/Game/GGJ/Mat/NS_BubblesSpawnEvier.NS_BubblesSpawnEvier" (`SceneComponent.K2_GetComponentLocation` (`self.NS_Bubbles`))))

(fn `InteractSpline`
  (params (BPC_InteractRef :type "/Game/GGJ/Blueprint/Interact/BPC_Interact Object Reference") (ValidParent :type "/Game/GGJ/Blueprint/Machines/BP_ParentMachines Object Reference"))
  (returns (MachinesHitted :type "/Game/GGJ/Blueprint/Machines/BP_ParentMachines Object Reference") (IsConnected :type Boolean))
  (return null false))

(fn `UserConstructionScript`)