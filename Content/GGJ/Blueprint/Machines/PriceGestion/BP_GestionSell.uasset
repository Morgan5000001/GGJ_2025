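; Manages item sell prices, loading starting entries from DT_FirstPrice at BeginPlay.
; A looping timer recalculates each price from its last value, circulating versus reference quantity, sensitivity and a fixed manipulation factor.
; Each new price is inserted at the front of that item's price history.
; FindItem is meant to look up an item's index but breaks after the first entry; the debug print on Tick is disconnected.
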(event `InitItemPrice`
  ;[1 1 1] InitPrice
  (bind _outrownames (`DataTableFunctionLibrary.GetDataTableRowNames` "/Game/GGJ/Blueprint/Machines/PriceGestion/DT_FirstPrice.DT_FirstPrice"))
  (for _array_element _outrownames
    (bind _returnvalue (`|GetDataTableRow` "/Game/GGJ/Blueprint/Machines/PriceGestion/DT_FirstPrice.DT_FirstPrice" _array_element)
      (:`then`
        (`KismetArrayLibrary.Array_Add` (`self.ItemPrices`) _returnvalue)))))

(event `self.ReceiveBeginPlay`
  (`self.InitItemPrice`)
  (`KismetSystemLibrary.K2_SetTimerDelegate` (delegate `TickPrice`) (`self.TimeTickPrice`) true))

(event `self.ReceiveTick`
  (params (DeltaSeconds :type "Float (single-precision)"))
  ;[0 0 0] Debug
  (for _array_element (`.Prices_3_1DF796354EDA1C2184CE21B4212AF658` (break `/Game/GGJ/Blueprint/Machines/PriceGestion/S_PreviousPrice` (`|GetArrayItem` (`self.ItemPrices`))))
    _))

(event `TickPrice`
  (bind _itemprices (`self.ItemPrices`))
  (for (_array_element _array_index) _itemprices
    (bind (_item _prices _number _quantiteref _facteurdesensibilite) (break `/Game/GGJ/Blueprint/Machines/PriceGestion/S_PreviousPrice` _array_element))
    (`KismetArrayLibrary.Array_Set` _itemprices _array_index (make `/Game/GGJ/Blueprint/Machines/PriceGestion/S_PreviousPrice` _item (`self.AddToPrice` _prices (`self.Price_Calculation` (`|GetArrayItem` _prices) _number _quantiteref _facteurdesensibilite 0.75)) _number _quantiteref _facteurdesensibilite))))

(fn `AddToPrice`
  (params (PreviousPrice :type "Array of Float (double-precision)") (NewPrice :type "Float (double-precision) (by ref)"))
  (returns (Price :type "Array of Float (double-precision)"))
  (locals (Local_PreviousPrice :type "Array of Float (double-precision)"))
  (bind _output_get (set `local.Local_PreviousPrice` PreviousPrice))
  (`KismetArrayLibrary.Array_Insert` _output_get NewPrice)
  (return (`local.Local_PreviousPrice`)))

(fn `FindItem`
  (params (ItemToCompare :type "/Game/GGJ/Blueprint/Machines/PriceGestion/S_PreviousPrice Structure"))
  (returns (`Contains?` :type Boolean) (Index :type Integer))
  (locals (Local_Find :type Boolean) (Local_IndexFind :type Integer))
  (for (_array_element _array_index) (`self.ItemPrices`)
    (if true
      (set `local.Local_Find` (`KismetStringLibrary.EqualEqual_StrStr` (`.Item_7_ACC9D24249BC52E901FF4C8268B8D2EA` (break `/Game/GGJ/Blueprint/Machines/PriceGestion/S_PreviousPrice` (`local.ItemToCompare`))) (`.Item_7_ACC9D24249BC52E901FF4C8268B8D2EA` (break `/Game/GGJ/Blueprint/Machines/PriceGestion/S_PreviousPrice` _array_element))))
      (set `local.Local_IndexFind` _array_index)
      (break)))
  (return (`local.Local_Find`) (`local.Local_IndexFind`)))

(fn `Price_Calculation`
  (params (LastPrice :type "Float (double-precision)") (QuantiteCirculation :type Integer) (QuantiteRef :type Integer :default 100) (FacteurDeSensibilite :type "Float (double-precision)" :default 1.0) (FacteurDeManipulation :type "Float (double-precision)" :default 1.0))
  (returns (Price :type "Float (double-precision)"))
  (return (* (`local.LastPrice`) (+ 1 (/ (- (`local.QuantiteRef`) (`local.QuantiteCirculation`)) (* (`local.QuantiteRef`) (`local.FacteurDeSensibilite`)))) (`local.FacteurDeManipulation`))))