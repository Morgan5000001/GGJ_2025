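; Bubble shaper machine for a game jam project that consumes its bubble count in a player-selected shape: round, square or triangle.
; Interacting cycles the shape enum and updates the preview mesh, except when wrapping to None.
; A one-second polling timer waits for IsItOkToStart, then starts a looping production timer whose interval shrinks with Level.
; Each production tick only decrements Bubbles and prints French debug text; no shaped bubble is spawned.
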(event `self.ReceiveBeginPlay`
  (bind _returnvalue (`KismetSystemLibrary.K2_SetTimerDelegate` (delegate `Is It ok to start?`) 1.0 true))
  (set `self.TimerStart` _returnvalue))

(event `/Game/GGJ/Blueprint/Interact/BPI_Interact.Interact`
  (if (> (`self.Shape`) 2)
    (set `self.Shape` "NewEnumerator0")
    (else
      (bind _output_get (set `self.Shape` (cast `/Game/GGJ/Blueprint/Inventory/E_BulleType` (+ (`self.Shape`) 1))))
      (`KismetSystemLibrary.PrintString` (`|GetEnumeratorNameAsString` _output_get))
      (`self.UpdateShape`))))

(event `Is It ok to start?`
  (if (`self.IsItOkToStart?`)
    (`KismetSystemLibrary.K2_ClearAndInvalidateTimerHandle` (`self.TimerStart`))
    (`self.Start Shaping`)
    (`KismetSystemLibrary.PrintString` (`KismetStringLibrary.Conv_IntToString` (`self.Bubbles`)))
    (else
      (`KismetSystemLibrary.K2_ClearAndInvalidateTimerHandle` (`self.TimerProd`)))))

(event `UpdateShape`
  (switch `/Game/GGJ/Blueprint/Inventory/E_BulleType` (`self.Shape`)
    (:`NewEnumerator1`
      (`StaticMeshComponent.SetStaticMesh` (`self.Shapes`) "/Game/FPWeapon/Mesh/FirstPersonProjectileMesh.FirstPersonProjectileMesh"))
    (:`NewEnumerator2`
      (`StaticMeshComponent.SetStaticMesh` (`self.Shapes`) "/Game/LevelPrototyping/Meshes/SM_Cube.SM_Cube"))
    (:`NewEnumerator3`
      (`StaticMeshComponent.SetStaticMesh` (`self.Shapes`) "/Game/LevelPrototyping/Meshes/SM_Ramp.SM_Ramp"))))

(event `Start Shaping`
  (bind _bubbles (`self.Bubbles`))
  (if (> _bubbles 0)
    (`KismetSystemLibrary.PrintString` (`KismetStringLibrary.Conv_IntToString` _bubbles))
    (bind _returnvalue (`KismetSystemLibrary.K2_SetTimerDelegate` (delegate `Send Bubbles`) (/ (`self.DefaultTime`) (`self.Level`)) true))
    (set `self.TimerProd` _returnvalue)
    (else
      (`KismetSystemLibrary.K2_ClearAndInvalidateTimerHandle` (`self.TimerProd`)))))

(event `Send Bubbles`
  (switch `/Game/GGJ/Blueprint/Inventory/E_BulleType` (`self.Shape`)
    (:`NewEnumerator1`
      (`self.SendRond`)
      (`KismetSystemLibrary.PrintString` "J'envoie un rond"))
    (:`NewEnumerator2`
      (`self.SendCarré`)
      (`KismetSystemLibrary.PrintString` "J'envoie un Carré"))
    (:`NewEnumerator3`
      (`self.SendTriangle`)
      (`KismetSystemLibrary.PrintString` "J'envoie un Triangle"))))

(event `SendRond`
  (`/Engine/EditorBlueprintResources/StandardMacros.DecrementInt` (`self.Bubbles`)))

(event `SendCarré`
  (`/Engine/EditorBlueprintResources/StandardMacros.DecrementInt` (`self.Bubbles`)))

(event `SendTriangle`
  (`/Engine/EditorBlueprintResources/StandardMacros.DecrementInt` (`self.Bubbles`)))

(fn `UserConstructionScript`)