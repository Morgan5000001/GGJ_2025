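; Level 1 bubble shaper machine that converts input items into items of its configured shape, keeping their color.
; On BeginPlay, StartMachine looks up the output in DT_Item using a row name built from shape plus input color.
; A looping timer, shortened by Level, moves one unit per tick from Before to Result.
; The timer clears when input runs out, output is full, or StopMachin is called.
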(event `self.ReceiveBeginPlay`
  (`self.StartMachine`))

(event `self.StartMachine`
  (bind _before (`self.Before`))
  (if (not (<= (`.Quantity_8_9749AB4D4EE8A746F67C62A14D2011B7` (break `/Game/GGJ/Blueprint/Inventory/S_Item` _before)) 0))
    (bind _returnvalue (`|GetDataTableRow` "/Game/GGJ/Blueprint/Inventory/DT_Item.DT_Item" (`KismetStringLibrary.Conv_StringToName` (`KismetStringLibrary.Concat_StrStr` (`|GetEnumeratorNameAsString` (`self.Shape`)) (`|GetEnumeratorNameAsString` (`.Color_5_CDCF0C03495CA6A2C3F344AB46A81A7A` (break `/Game/GGJ/Blueprint/Inventory/S_Item` _before))))))
      (:`then`
        (bind (_type _color _quantity _icon) (break `/Game/GGJ/Blueprint/Inventory/S_Item` _returnvalue))
        (set `self.Result` (make `/Game/GGJ/Blueprint/Inventory/S_Item` _type _color 0 _icon))
        (bind _returnvalue_2 (`KismetSystemLibrary.K2_SetTimerDelegate` (delegate `ModifiedBubble`) (/ (`self.TIME`) (`self.Level`)) true))
        (set `self.NEEDTOUSE` _returnvalue_2)))))

(event `ModifiedBubble`
  (bind _before (`self.Before`))
  (bind _result (`self.Result`))
  (if (not (or (< (- (`.Quantity_8_9749AB4D4EE8A746F67C62A14D2011B7` (break `/Game/GGJ/Blueprint/Inventory/S_Item` (`self.Before`))) 1) 0) (> (+ (`.Quantity_8_9749AB4D4EE8A746F67C62A14D2011B7` (break `/Game/GGJ/Blueprint/Inventory/S_Item` (`self.Result`))) 1) (`self.MaxQuantityResult`))))
    (bind _structout (setmembers `/Game/GGJ/Blueprint/Inventory/S_Item` :`StructRef` _before :`Quantity` (- (`.Quantity_8_9749AB4D4EE8A746F67C62A14D2011B7` (break `/Game/GGJ/Blueprint/Inventory/S_Item` _before)) 1)))
    (set `self.Before` _structout)
    (bind _structout_2 (setmembers `/Game/GGJ/Blueprint/Inventory/S_Item` :`StructRef` _result :`Quantity` (+ (`.Quantity_8_9749AB4D4EE8A746F67C62A14D2011B7` (break `/Game/GGJ/Blueprint/Inventory/S_Item` _result)) 1)))
    (set `self.Result` _structout_2)
    (else
      (`KismetSystemLibrary.K2_ClearAndInvalidateTimerHandle` (`self.NEEDTOUSE`))
      (`/Engine/EditorBlueprintResources/StandardMacros.IsValid` (`self.WBP_WidgetRef`)))))

(event `self.StopMachin`
  (`KismetSystemLibrary.K2_ClearAndInvalidateTimerHandle` (`self.NEEDTOUSE`)))

(fn `UserConstructionScript`)