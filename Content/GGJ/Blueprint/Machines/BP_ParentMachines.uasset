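; Base machine Blueprint that produces bubbles into its Result stock and passes them along pipes to other machines.
; Server events run a looping timer, scaled by Level, to add bubbles up to a maximum.
; InteractSpline links a parent machine to this one with a BP_Spline; the parent then moves one item per second into this machine's Before slot.
; Interact saves the player's inventory to the GameInstance and toggles the WBP_Machines widget.
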(event `self.ReceiveBeginPlay`)

(event `RS_TakeMachin`
  (params (NewParam :type "/Game/GGJ/Blueprint/Machines/BP_ParentMachines Object Reference"))
  (bind _structout (setmembers `/Game/GGJ/Blueprint/Inventory/S_Item` :`StructRef` (`/Game/GGJ/Blueprint/Machines/BP_ParentMachines.Result` NewParam) :`Quantity` 0))
  (set `/Game/GGJ/Blueprint/Machines/BP_ParentMachines.Result` _structout NewParam)
  (`KismetSystemLibrary.PrintString` (`KismetSystemLibrary.GetDisplayName` NewParam) true true (struct :`R` 1.0 :`B` 0.831473 :`A` 1.0) 20.0))

(event `RS_StartMachine`
  ;[1 1 1] Creation de bulles Replique
  (bind _returnvalue (`KismetSystemLibrary.K2_SetTimerDelegate` (`|CreateDelegate` :!event `RS_StartCreatingBubbles`) (/ (`self.TIME`) (`self.Level`)) true))
  (set `self.TimerCreatingBubbles` _returnvalue))

(event `RS_StartCreatingBubbles`
  (bind _returnvalue (+ (`.Quantity_8_9749AB4D4EE8A746F67C62A14D2011B7` (break `/Game/GGJ/Blueprint/Inventory/S_Item` (`self.Result`))) 1))
  ;[1 1 1] Creation de bulles Replique
  (if (not (> _returnvalue (`self.MaxQuantityResult`)))
    (setmembers `/Game/GGJ/Blueprint/Inventory/S_Item` :`StructRef` (`self.Result`) :`Quantity` _returnvalue) ; Pour ne modifer que la quantite et pas toute la structure
    (else
      (`self.RS_StopMachin`))))

(event `RS_StopMachin`
  ;[1 1 1] Creation de bulles Replique
  (`KismetSystemLibrary.K2_ClearAndInvalidateTimerHandle` (`self.TimerCreatingBubbles`)))

(event `self.ReceiveTick`
  (params (DeltaSeconds :type "Float (single-precision)"))
  ;[0 0 0] Debug
)

(event `Connected`
  (params (Batiment :type "/Game/GGJ/Blueprint/Machines/BP_ParentMachines Object Reference"))
  (set `self.BatimentLinked` Batiment)
  (bind _returnvalue (`KismetSystemLibrary.K2_SetTimerDelegate` (delegate `Add`) 1.0 true))
  (set `self.NewVar` _returnvalue))

(event `Add`
  (bind _result (`self.Result`))
  (bind (_result_type _result_color _result_quantity _result_icon) (break `/Game/GGJ/Blueprint/Inventory/S_Item` (`self.Result`)))
  (bind _result_2 (`self.Result`))
  (bind _result_3 (`self.Result`))
  (bind _batimentlinked (`self.BatimentLinked`))
  (bind _before (`/Game/GGJ/Blueprint/Machines/BP_ParentMachines.Before` _batimentlinked))
  (if (not (< (- (`.Quantity_8_9749AB4D4EE8A746F67C62A14D2011B7` (break `/Game/GGJ/Blueprint/Inventory/S_Item` _result)) 1) 0))
    (if (`/Game/GGJ/Blueprint/Inventory/BFL_InventoryGestion.CompareItem` _result (`/Game/GGJ/Blueprint/Machines/BP_ParentMachines.Before` (`self.BatimentLinked`)))
      (bind _structout (setmembers `/Game/GGJ/Blueprint/Inventory/S_Item` :`StructRef` _result_3 :`Quantity` (- (`.Quantity_8_9749AB4D4EE8A746F67C62A14D2011B7` (break `/Game/GGJ/Blueprint/Inventory/S_Item` _result_3)) 1)))
      (set `self.Result` _structout)
      (bind _structout_2 (setmembers `/Game/GGJ/Blueprint/Inventory/S_Item` :`StructRef` _before :`Quantity` (+ (`.Quantity_8_9749AB4D4EE8A746F67C62A14D2011B7` (break `/Game/GGJ/Blueprint/Inventory/S_Item` _before)) 1)))
      (set `/Game/GGJ/Blueprint/Machines/BP_ParentMachines.Before` _structout_2 _batimentlinked)
      (else
        (bind _structout_3 (setmembers `/Game/GGJ/Blueprint/Inventory/S_Item` :`StructRef` _before :`Type` _result_type :`Color` _result_color :`Quantity` 1 :`Icon` _result_icon))
        (set `/Game/GGJ/Blueprint/Machines/BP_ParentMachines.Before` _structout_3 _batimentlinked)
        (bind _structout_4 (setmembers `/Game/GGJ/Blueprint/Inventory/S_Item` :`StructRef` _result_2 :`Quantity` (- (`.Quantity_8_9749AB4D4EE8A746F67C62A14D2011B7` (break `/Game/GGJ/Blueprint/Inventory/S_Item` _result_2)) 1)))
        (set `self.Result` _structout_4)))))

(event `/Game/GGJ/Blueprint/Interact/BPI_Interact.Interact`
  (params (PlayerRef :type "/Game/GGJ/Blueprint/FirstPerson/Blueprints/BP_FirstPersonCharacter Object Reference"))
  (bind _returnvalue (`GameplayStatics.GetPlayerController` 0))
  (bind _bp_inventory (`/Game/GGJ/Blueprint/FirstPerson/Blueprints/BP_FirstPersonCharacter.BP_Inventory` PlayerRef))
  (`/Game/GGJ/Blueprint/GI_CustomGameInstance.SaveInventory` (cast `/Game/GGJ/Blueprint/GI_CustomGameInstance` (`GameplayStatics.GetGameInstance`) :!pure true) "" (`/Game/GGJ/Blueprint/Inventory/BP_Inventory.Inventory` _bp_inventory))
  (`/Engine/EditorBlueprintResources/StandardMacros.IsValid` (`self.WBP_WidgetRef`)
    (:`Is Valid`
      (`Widget.RemoveFromParent` (`self.WBP_WidgetRef`))
      (set `self.WBP_WidgetRef` null)
      (`WidgetBlueprintLibrary.SetInputMode_GameOnly` _returnvalue true)
      (set `PlayerController.bShowMouseCursor` false _returnvalue))
    (:`Is Not Valid`
      (bind _returnvalue_2 (`|CreateWidget` "/Game/GGJ/Widget/WBP_Machines.WBP_Machines_C" null (`self.TypeBuild`) self (`self.Result`) (`self.Before`) _bp_inventory))
      (bind _output_get (set `self.WBP_WidgetRef` _returnvalue_2))
      (`UserWidget.AddToViewport` _output_get 0))))

(fn `InteractSpline`
  (params (BP_BuildComponentRef :type "/Game/GGJ/Blueprint/BuildMode/BP_BuildComponent Object Reference") (ValidParent :type "/Game/GGJ/Blueprint/Machines/BP_ParentMachines Object Reference"))
  (returns (MachinesHitted :type "/Game/GGJ/Blueprint/Machines/BP_ParentMachines Object Reference") (IsConnected :type Boolean))
  (`/Engine/EditorBlueprintResources/StandardMacros.IsValid` ValidParent
    (:`Is Valid`
      (bind _output_get (set `self.ConnectedMachin` ValidParent))
      (`self.Connected` _output_get self)
      (`|SpawnActorFromClass` "/Game/GGJ/Blueprint/Machines/BP_Spline.BP_Spline_C" (`KismetMathLibrary.MakeTransform` (`SceneComponent.K2_GetComponentLocation` (`self.PivotPipe`))) "Undefined" "MultiplyWithRoot" null (`SceneComponent.K2_GetComponentLocation` (`/Game/GGJ/Blueprint/Machines/BP_ParentMachines.PivotPipe` (`local.ValidParent`))) _output_get null)
      (set `/Game/GGJ/Blueprint/BuildMode/BP_BuildComponent.LastBat` null BP_BuildComponentRef)
      (return self true))
    (:`Is Not Valid`
      (return self false))))

(fn `UserConstructionScript`)