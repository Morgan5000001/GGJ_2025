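; Bubble maker machine that periodically produces a round normal bubble item into its result inventory.
; A looping one-second timer, started on BeginPlay or MachineIsOn, adds one bubble up to a cap of three and refreshes the linked widget.
; A level-scaled time is computed, but the timer ignores it.
; The on/off toggle that shows Niagara or clears timers is unconnected and never runs.
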(event `self.ReceiveBeginPlay`
  ;[1 1 1] Si le caca est cuit, alors :
  (set `self.NewTime` (/ (`self.Defaul time`) (`self.Level`)) :!label _label)
  (bind _returnvalue (`KismetSystemLibrary.K2_SetTimerDelegate` (delegate `Start Creating Bubbles`) 1.0 true))
  ;;[1 1 1] Le temps
  (set `self.Timer` _returnvalue))

(event `Machine Is On`
  ;[1 1 1] Si le caca est cuit, alors :
  (goto _label))

(event `Start Creating Bubbles`
  (bind _wbp_widgetref (`self.WBP_WidgetRef`))
  ;[1 1 1] Si le caca est cuit, alors :
  (bind _return_inventory (`/Game/GGJ/Blueprint/Inventory/BFL_InventoryGestion.AddItemInventory` (make `/Game/GGJ/Blueprint/Inventory/S_Item` "NewEnumerator1" "NewEnumerator1" 0 "/Game/GGJ/Image/Bubbles/Round/MI_RoundNormalBubble.MI_RoundNormalBubble") 1 (`self.ResultInventoryMachin`) 3))
  (set `self.ResultInventoryMachin` _return_inventory)
  (`/Engine/EditorBlueprintResources/StandardMacros.IsValid` _wbp_widgetref
    (:`Is Valid`
      (`/Game/GGJ/Widget/WBP_Machines.RefreshDataResult` _wbp_widgetref (`self.ResultInventoryMachin`)))))

(fn `UserConstructionScript`)