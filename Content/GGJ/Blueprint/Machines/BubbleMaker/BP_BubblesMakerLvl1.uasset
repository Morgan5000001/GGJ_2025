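; BP_BubblesMakerLvl1 is a bubble-maker machine that produces its result item on a looping timer.
; The timer starts on BeginPlay or StartMachine, with its interval set to a base time divided by the machine's Level.
; Each tick adds one to the result quantity; when another would exceed the maximum, StopMachin clears the stored timer handle.
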(event `self.ReceiveBeginPlay`
  ;[1 1 1] Si le caca est cuit, alors :
  (bind _output_get (set `self.NewTime` (/ (`self.TIME`) (`self.Level`)) :!label _label))
  (bind _returnvalue (`KismetSystemLibrary.K2_SetTimerDelegate` (delegate `Start Creating Bubbles`) _output_get true))
  ;;[1 1 1] Le temps
  (set `self.NEEDTOUSE` _returnvalue))

(event `self.StartMachine`
  ;[1 1 1] Si le caca est cuit, alors :
  (goto _label))

(event `Start Creating Bubbles`
  (bind _result (`self.Result`))
  (bind _returnvalue (+ (`.Quantity_8_9749AB4D4EE8A746F67C62A14D2011B7` (break `/Game/GGJ/Blueprint/Inventory/S_Item` _result)) 1))
  ;[1 1 1] Si le caca est cuit, alors :
  (if (not (> _returnvalue (`self.MaxQuantityResult`)))
    (setmembers `/Game/GGJ/Blueprint/Inventory/S_Item` :`StructRef` _result :`Quantity` _returnvalue)
    (else
      (`self.StopMachin`))))

(event `self.StopMachin`
  (`KismetSystemLibrary.K2_ClearAndInvalidateTimerHandle` (`self.NEEDTOUSE`)))

(fn `UserConstructionScript`)