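; Sell machine where the player opens an inventory screen to sell items at fluctuating prices.
; A looping timer multiplies each reference price by a curve, picked at random per item whenever the 0–10 step index restarts, keeping the previous prices.
; Interact toggles the camera blend, cursor and WBP_InventorySell widget, guarded against re-triggering mid-blend, and notifies the player's tutorial component if present.
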(event `self.ReceiveBeginPlay`
  (`parent.ReceiveBeginPlay`)
  (`KismetSystemLibrary.K2_SetTimerDelegate` (delegate `CustomEvent`) (`self.TickDeLectureDeCurve`) true))

(event `CustomEvent`
  (bind _referenceitemprice (`self.ReferenceItemPrice`))
  (bind _indexcurve (`self.IndexCurve`))
  (set `self.PreviousItems` (`self.AllItems`))
  (bind _keys (`BlueprintMapLibrary.Map_Keys` _referenceitemprice))
  (bind _values (`BlueprintMapLibrary.Map_Values` _referenceitemprice))
  (for (_array_element _array_index) _keys
    (if (== (`self.IndexCurve`) 0)
      (bind _output_get (set `self.NewVar_0` (`KismetArrayLibrary.Array_Random` (`self.Curve`))))
      (`BlueprintMapLibrary.Map_Add` (`self.CurveSelected`) _array_element _output_get)
      (bind _output (`|GetArrayItem` _values _array_index))
      (`BlueprintMapLibrary.Map_Add` (`self.AllItems`) _array_element (* _output (`CurveFloat.GetFloatValue` (`self.NewVar_0`) (`KismetMathLibrary.Conv_IntToDouble` (`self.IndexCurve`)))))
      (else
        (`BlueprintMapLibrary.Map_Add` (`self.AllItems`) _array_element (* (`CurveFloat.GetFloatValue` (`BlueprintMapLibrary.Map_Find` (`self.CurveSelected`) _array_element) (`KismetMathLibrary.Conv_IntToDouble` (`self.IndexCurve`))) _output)))))
  (if (== _indexcurve 10)
    (set `self.IndexCurve` 0)
    (else
      (`/Engine/EditorBlueprintResources/StandardMacros.IncrementInt` _indexcurve))))

(event `/Game/GGJ/Blueprint/Interact/BPI_Interact.Interact`
  (params (PlayerRef :type "/Game/GGJ/Blueprint/FirstPerson/Blueprints/BP_FirstPersonCharacter Object Reference"))
  (bind _returnvalue (`self.GetComponentByClass` PlayerRef "/Game/Blueprints/Tutoriel/BP_Tutoriel.BP_Tutoriel_C"))
  (`|ExecutionSequence`
    (:`then_0`
      (if (`self.EndBlend?`)
        (if (not (`self.SellInvnetoryOpen?`))
          (set `PlayerController.bShowMouseCursor` true (`GameplayStatics.GetPlayerController` 0))
          (set `self.EndBlend?` false)
          (`PlayerController.SetViewTargetWithBlend` (`GameplayStatics.GetPlayerController` 0) self 0.5 "VTBlend_Linear" 0.0 false)
          (set `self.SellInvnetoryOpen?` true)
          (`KismetSystemLibrary.Delay` 0.5)
          (bind _output_get (set `self.Player Ref` PlayerRef))
          (bind _returnvalue_2 (`|CreateWidget` "/Game/GGJ/Widget/WBP_InventorySell.WBP_InventorySell_C" null (`/Game/GGJ/Blueprint/Inventory/BP_Inventory.Inventory` (`/Game/GGJ/Blueprint/FirstPerson/Blueprints/BP_FirstPersonCharacter.BP_Inventory` PlayerRef)) self _output_get))
          (bind _output_get_2 (set `self.RefSellWidget` _returnvalue_2))
          (`UserWidget.AddToViewport` _output_get_2 0)
          (set `self.EndBlend?` true)
          (else
            (set `self.EndBlend?` false)
            (`Widget.RemoveFromParent` (`self.RefSellWidget`))
            (set `PlayerController.bShowMouseCursor` false (`GameplayStatics.GetPlayerController` 0))
            (`PlayerController.SetViewTargetWithBlend` (`GameplayStatics.GetPlayerController` 0) PlayerRef 0.5 "VTBlend_Linear" 0.0 false)
            (`KismetSystemLibrary.Delay` 0.5)
            (set `self.SellInvnetoryOpen?` false)
            (set `self.EndBlend?` true)))))
    (:`then_1`
      (`/Engine/EditorBlueprintResources/StandardMacros.IsValid` _returnvalue
        (:`Is Valid`
          (message `/Game/Blueprints/Tutoriel/BPi_Tutoriel.InteractTablette` _returnvalue))))))

(fn `UserConstructionScript`
  (`parent.UserConstructionScript`))