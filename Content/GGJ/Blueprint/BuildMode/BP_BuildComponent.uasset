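; Player build-mode component for placing, linking and selling bubble factory machines and pipes bought with gold.
; It loads DT_Build into a scrollable inventory and previews the selected mesh via a per-tick camera trace, with manual rotation.
; Gold, floor tag and sphere-trace overlap checks set preview validity and material, while pipes must target machines.
; Placing spawns machines or starts spline links, selling refunds half price, and both update game-instance saves.
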(event `self.ReceiveBeginPlay`
  (bind _outrownames (`DataTableFunctionLibrary.GetDataTableRowNames` "/Game/GGJ/Blueprint/Machines/DT_Build.DT_Build"))
  (for _array_element _outrownames
    (bind _returnvalue (`|GetDataTableRow` "/Game/GGJ/Blueprint/Machines/DT_Build.DT_Build" _array_element)
      (:`then`
        (`KismetArrayLibrary.Array_Add` (`self.Inventory`) _returnvalue)))))

(event `self.ReceiveTick`
  (params (DeltaSeconds :type "Float (single-precision)"))
  (if (`self.BuildMode ?`)
    (`self.PreviewLoop`)))

(event `EnhancedInput|/Game/GGJ/Blueprint/FirstPerson/Input/Actions/IA_BuildMode`
  (params (ActionValue :type Boolean) (ElapsedSeconds :type "Float (double-precision)") (TriggeredSeconds :type "Float (double-precision)") (InputAction :type "InputAction Object Reference" :default "/Game/GGJ/Blueprint/FirstPerson/Input/Actions/IA_BuildMode.IA_BuildMode"))
  (:`Started`
    (if (`self.AnimReset?`)
      (if (not (`self.BuildMode ?`))
        (`/Game/GGJ/Widget/WBP_InterfacePlayer.OpenBuildMode` (`/Game/GGJ/Blueprint/FirstPerson/Blueprints/BP_FirstPersonCharacter.WidgetInterface` (`self.PlayerRef`)))
        (else
          (`/Game/GGJ/Widget/WBP_InterfacePlayer.CloseBuildMode` (`/Game/GGJ/Blueprint/FirstPerson/Blueprints/BP_FirstPersonCharacter.WidgetInterface` (`self.PlayerRef`))))))))

(event `StopDropModeWidget`
  (set `self.BuildMode ?` false)
  (bind _previewmesh (`self.PreviewMesh`)
    (:`then`
      (`StaticMeshComponent.SetStaticMesh` _previewmesh null)
      (set `self.PreviewMesh` null)
      (`self.Reset Drop Mode`))
    (:`else`)))

(event `Reset Drop Mode`
  (bind _previewmesh (`self.PreviewMesh`))
  ;[0.01938 0.01938 0.01938] Line Trace Preview Mesh
  (goto _label :!via `Reset`))

(event `SetMaterial`
  (params (Target :type "PrimitiveComponent Object Reference") (Material :type "MaterialInterface Object Reference"))
  ;[0.01938 0.01938 0.01938] Line Trace Preview Mesh
  (`PrimitiveComponent.SetMaterial` Target 0 Material)
  (`PrimitiveComponent.SetMaterial` Target 1 Material))

(event `PreviewLoop`
  (bind _previewmesh (`self.PreviewMesh`))
  (bind _drop_preview_transform_location (`KismetMathLibrary.BreakTransform` (`self.Drop Preview Transform`)))
  (bind (_returnvalue_location _returnvalue_rotation) (`KismetMathLibrary.BreakTransform` (`SceneComponent.K2_GetComponentToWorld` (`GGJ_2025Character.FirstPersonCameraComponent` (`self.PlayerRef`)))))
  ;[0.01938 0.01938 0.01938] Line Trace Preview Mesh
  (`|ExecutionSequence`
    (:`then_0`
      (bind (_outhit _returnvalue) (`KismetSystemLibrary.LineTraceSingle` :`Start` _returnvalue_location :`End` (+ _returnvalue_location (* (`KismetMathLibrary.GetForwardVector` _returnvalue_rotation) (`self.DistanceToDrop`))) :`TraceChannel` "TraceTypeQuery1" :`DrawDebugType` "ForOneFrame"))
      (if _returnvalue
        (set `self.CanDrop?` true)
        (`|ExecutionSequence`
          (:`then_0`
            (`/Engine/EditorBlueprintResources/StandardMacros.DoOnce` false :!label _label
              (:`Completed`
                (bind _returnvalue_2 (`|AddComponentByClass` (`self.PlayerRef`) "/Script/Engine.StaticMeshComponent" false (`self.Drop Preview Transform`)))
                (bind _output_get (set `self.PreviewMesh` _returnvalue_2))
                (`StaticMeshComponent.SetStaticMesh` _output_get (`.StaticMesh_11_A84BA1F745AE8A56CB8CA4BB3F9D264D` (break `/Game/GGJ/Blueprint/Machines/S_Build` (`|GetArrayItem` (`self.Inventory`) (`self.SelectIndex`)))))
                (`self.SetMaterial` _previewmesh (`self.MaterialTrue`))
                (`PrimitiveComponent.SetCollisionObjectType` _previewmesh "ECC_WorldStatic")
                (`PrimitiveComponent.SetCollisionEnabled` _previewmesh "QueryAndPhysics"))))
          (:`then_1`
            (bind (_bblockinghit _binitialoverlap _time _distance _location _impactpoint _normal _impactnormal _physmat _hitactor) (`GameplayStatics.BreakHitResult` _outhit))
            (set `self.HitMachines` _hitactor)
            (bind _output_get_2 (set `self.Drop Preview Transform` (`KismetMathLibrary.MakeTransform` _location (`KismetMathLibrary.MakeRotator` 0.0 0.0 (`self.Drop Preview Transform Rotation Y (Pitch)`)))))
            (`SceneComponent.K2_SetWorldTransform` (`self.PreviewMesh`) _output_get_2 false false)
            (if (== (`.BpToSpawn_13_7035BA9D4ED25A7BECDA8AA6AF64B210` (break `/Game/GGJ/Blueprint/Machines/S_Build` (`|GetArrayItem` (`self.Inventory`) (`self.SelectIndex`)))) "/Game/GGJ/Blueprint/Machines/BP_Spline.BP_Spline_C") :!label _label_2
              (bind _asbp_parent_machines (cast `/Game/GGJ/Blueprint/Machines/BP_ParentMachines` _hitactor)
                (:`then`
                  (switch `/Game/GGJ/Blueprint/Machines/E_TypeBuild` (`/Game/GGJ/Blueprint/Machines/BP_ParentMachines.TypeBuild` _asbp_parent_machines)
                    (:`NewEnumerator0`
                      (set `self.CanDrop?` false :!label _label_3)
                      (bind _previewmesh_2 (`self.PreviewMesh`)
                        (:`then`
                          (`self.SetMaterial` _previewmesh_2 (`self.MaterialWrong`)))
                        (:`else`)))
                    (:`NewEnumerator1`
                      (set `self.CanDrop?` true :!label _label_4)
                      (bind _previewmesh_3 (`self.PreviewMesh`)
                        (:`then`
                          (`self.SetMaterial` _previewmesh_3 (`self.MaterialTrue`)))
                        (:`else`)))
                    (:`NewEnumerator2`
                      (goto _label_4))
                    (:`NewEnumerator3`
                      (goto _label_4))
                    (:`NewEnumerator4`
                      (goto _label_3))))
                (:`CastFailed`
                  (goto _label_3)))
              (elif (and (>= (`/Game/GGJ/Blueprint/FirstPerson/Blueprints/BP_FirstPersonCharacter.Gold` (`self.PlayerRef`)) (`.Price_6_5A054677451A8E53069F469202B1236B` (break `/Game/GGJ/Blueprint/Machines/S_Build` (`|GetArrayItem` (`self.Inventory`) (`self.SelectIndex`))))) (not (`self.OverlapPreview?`)) (`Actor.ActorHasTag` (`self.HitMachines`) "Floor"))
                (goto _label_4)
                (else
                  (goto _label_3))))))
        (else
          (bind _previewmesh_4 (`self.PreviewMesh`)
            (:`then`
              (bind (_returnvalue_x _returnvalue_y) (`KismetMathLibrary.BreakVector` (`SceneComponent.K2_GetComponentLocation` _previewmesh_4)))
              (bind _output_get_3 (set `self.Drop Preview Transform` (`KismetMathLibrary.MakeTransform` (`KismetMathLibrary.MakeVector` _returnvalue_x _returnvalue_y) (`KismetMathLibrary.MakeRotator` 0.0 0.0 (`self.Drop Preview Transform Rotation Y (Pitch)`)))))
              (`SceneComponent.K2_SetWorldTransform` (`self.PreviewMesh`) _output_get_3 false false)
              (goto _label_2))
            (:`else`
              (goto _label_2))))))
    (:`then_1`
      (`self.PreviewMesh`
        (:`then`
          (bind (_outhits _returnvalue_3) (`KismetSystemLibrary.SphereTraceMulti` :`Start` _drop_preview_transform_location :`End` _drop_preview_transform_location :`Radius` (`.RadiusCollision_22_E309E0BE4D952D658A3DB3ADFC283CA6` (break `/Game/GGJ/Blueprint/Machines/S_Build` (`|GetArrayItem` (`self.Inventory`) (`self.SelectIndex`)))) :`TraceChannel` "TraceTypeQuery1" :`DrawDebugType` "ForOneFrame" :`bIgnoreSelf` false))
          (if _returnvalue_3
            (for _array_element _outhits
              (bind (_bblockinghit_2 _binitialoverlap_2 _time_2 _distance_2 _location_2 _impactpoint_2 _normal_2 _impactnormal_2 _physmat_2 _hitactor_2 _hitcomponent) (`GameplayStatics.BreakHitResult` _array_element))
              (if (or (`Actor.ActorHasTag` _hitactor_2 "Floor") (== _hitcomponent (`self.PreviewMesh`)))
                (set `self.OverlapPreview?` false)
                (else
                  (set `self.OverlapPreview?` true)
                  (break))))))
        (:`else`)))))

(event `EnhancedInput|/Game/GGJ/Blueprint/FirstPerson/Input/Actions/IA_Scroll`
  (params (ActionValue :type "Float (double-precision)") (ElapsedSeconds :type "Float (double-precision)") (TriggeredSeconds :type "Float (double-precision)") (InputAction :type "InputAction Object Reference" :default "/Game/GGJ/Blueprint/FirstPerson/Input/Actions/IA_Scroll.IA_Scroll"))
  (bind _selectindex (`self.SelectIndex`))
  (bind _widgetinterface (`/Game/GGJ/Blueprint/FirstPerson/Blueprints/BP_FirstPersonCharacter.WidgetInterface` (`self.PlayerRef`)))
  ;[1 1 1] Switch build
  (:`Started`
    (if (`self.BuildMode ?`)
      (set `self.MaxItem` (- (`KismetArrayLibrary.Array_Length` (`self.Inventory`)) 1))
      (if (== ActionValue -1.0)
        (if (== (`self.SelectIndex`) (`self.MaxItem`))
          (set `self.SelectIndex` 0)
          (else
            (`/Engine/EditorBlueprintResources/StandardMacros.IncrementInt` _selectindex
              (:`  `
                _))))
        (elif (== (`self.SelectIndex`) 0)
          (set `self.SelectIndex` (`self.MaxItem`))
          (else
            (`/Engine/EditorBlueprintResources/StandardMacros.DecrementInt` _selectindex
              (:`  `
                _)))))
      (if (`self.BuildMode ?`)
        (bind _previewmesh (`self.PreviewMesh`)
          (:`then`
            (`StaticMeshComponent.SetStaticMesh` _previewmesh (`.StaticMesh_11_A84BA1F745AE8A56CB8CA4BB3F9D264D` (break `/Game/GGJ/Blueprint/Machines/S_Build` (`|GetArrayItem` (`self.Inventory`) (`self.SelectIndex`)))))
            (`GameplayStatics.PlaySound2D` "/Game/Free_UI/CUE/Minimalist1_Cue.Minimalist1_Cue" 1.0 1.0 0.0 null null)
            (`Widget.SetUserFocus` (`/Game/GGJ/Widget/WBP_Build.Button_1` (`|GetArrayItem` (`/Game/GGJ/Widget/WBP_InterfacePlayer.WidgetBuildAll` _widgetinterface) (`self.SelectIndex`))) (`GameplayStatics.GetPlayerController` 0))
            (`ScrollBox.SetScrollWhenFocusChanges` (`/Game/GGJ/Widget/WBP_InterfacePlayer.ScrollBox_0` _widgetinterface) "AnimatedScroll"))
          (:`else`))))))

(event `EnhancedInput|/Game/GGJ/Blueprint/FirstPerson/Input/Actions/IA_RotatePreview`
  (params (ActionValue :type Boolean) (ElapsedSeconds :type "Float (double-precision)") (TriggeredSeconds :type "Float (double-precision)") (InputAction :type "InputAction Object Reference" :default "/Game/GGJ/Blueprint/FirstPerson/Input/Actions/IA_RotatePreview.IA_RotatePreview"))
  ;[1 1 1] Rotate preview
  (:`Triggered`
    (set `self.Drop Preview Transform Rotation Y (Pitch)` (+ (`self.Drop Preview Transform Rotation Y (Pitch)`) 1.0))))

(event `EnhancedInput|/Game/GGJ/Blueprint/FirstPerson/Input/Actions/IA_PlaceItem`
  (params (ActionValue :type Boolean) (ElapsedSeconds :type "Float (double-precision)") (TriggeredSeconds :type "Float (double-precision)") (InputAction :type "InputAction Object Reference" :default "/Game/GGJ/Blueprint/FirstPerson/Input/Actions/IA_PlaceItem.IA_PlaceItem"))
  (bind (_drop_preview_transform_location _drop_preview_transform_rotation _drop_preview_transform_scale) (`KismetMathLibrary.BreakTransform` (`self.Drop Preview Transform`)))
  (bind _playerref (`self.PlayerRef`))
  (bind _returnvalue (`Actor.GetComponentByClass` (`self.PlayerRef`) "/Game/Blueprints/Tutoriel/BP_Tutoriel.BP_Tutoriel_C"))
  (bind _asgi_custom_game_instance (cast `/Game/GGJ/Blueprint/GI_CustomGameInstance` (`GameplayStatics.GetGameInstance`) :!pure true))
  (bind (_itemname _price _staticmesh _bptospawn) (break `/Game/GGJ/Blueprint/Machines/S_Build` (`|GetArrayItem` (`self.Inventory`) (`self.SelectIndex`))))
  ;[0.01938 0.01938 0.01938] Place Build
  (:`Started`
    (if (and (`self.BuildMode ?`) (`self.CanDrop?`))
      (if (>= (- (`/Game/GGJ/Blueprint/FirstPerson/Blueprints/BP_FirstPersonCharacter.Gold` (`self.PlayerRef`)) (`.Price_6_5A054677451A8E53069F469202B1236B` (break `/Game/GGJ/Blueprint/Machines/S_Build` (`|GetArrayItem` (`self.Inventory`) (`self.SelectIndex`))))) 0.0)
        (if (not (== _bptospawn "/Game/GGJ/Blueprint/Machines/BP_Spline.BP_Spline_C"))
          (bind _returnvalue_2 (`|SpawnActorFromClass` _bptospawn (`KismetMathLibrary.MakeTransform` _drop_preview_transform_location _drop_preview_transform_rotation _drop_preview_transform_scale) "AlwaysSpawn" "MultiplyWithRoot" null null))
          (bind _output_get (set `/Game/GGJ/Blueprint/FirstPerson/Blueprints/BP_FirstPersonCharacter.Gold` (- (`/Game/GGJ/Blueprint/FirstPerson/Blueprints/BP_FirstPersonCharacter.Gold` _playerref) (`.Price_6_5A054677451A8E53069F469202B1236B` (break `/Game/GGJ/Blueprint/Machines/S_Build` (`|GetArrayItem` (`self.Inventory`) (`self.SelectIndex`))))) _playerref))
          (`/Game/GGJ/Blueprint/GI_CustomGameInstance.SaveBatAdd` _asgi_custom_game_instance null (`KismetMathLibrary.MakeTransform` _drop_preview_transform_location _drop_preview_transform_rotation _drop_preview_transform_scale))
          (`/Game/GGJ/Blueprint/GI_CustomGameInstance.SaveGold` _asgi_custom_game_instance _output_get)
          (`GameplayStatics.PlaySound2D` "/Game/UI_SFX_Free_Pack/Cues/Purchase/coins_70_Cue.coins_70_Cue" 1.0 1.0 0.0 null null)
          (`/Engine/EditorBlueprintResources/StandardMacros.IsValid` _returnvalue
            (:`Is Valid`
              (message `/Game/Blueprints/Tutoriel/BPi_Tutoriel.PlaceUsine` _returnvalue)
              (`NiagaraFunctionLibrary.SpawnSystemAtLocation` "/Game/GGJ/Mat/NS_Sell.NS_Sell" (`SceneComponent.K2_GetComponentLocation` (`/Game/GGJ/Blueprint/Machines/BP_ParentMachines.Machine` _returnvalue_2)))))
          (else
            (`KismetSystemLibrary.PrintString` "TEST")
            (bind (_machineshitted _isconnected) (message `/Game/GGJ/Blueprint/Interact/BPI_Interact.InteractSpline` (`self.HitMachines`) self (`self.LastBat`)))
            (if (not _isconnected)
              (set `self.LastBat` _machineshitted))))))))

(event `EnhancedInput|/Game/GGJ/Blueprint/FirstPerson/Input/Actions/IA_SellBuild`
  (params (ActionValue :type Boolean) (ElapsedSeconds :type "Float (double-precision)") (TriggeredSeconds :type "Float (double-precision)") (InputAction :type "InputAction Object Reference" :default "/Game/GGJ/Blueprint/FirstPerson/Input/Actions/IA_SellBuild.IA_SellBuild"))
  (bind _playerref (`self.PlayerRef`))
  (bind _playerref_2 (`self.PlayerRef`))
  (bind _asgi_custom_game_instance (cast `/Game/GGJ/Blueprint/GI_CustomGameInstance` (`GameplayStatics.GetGameInstance`) :!pure true))
  (bind (_returnvalue_location _returnvalue_rotation) (`KismetMathLibrary.BreakTransform` (`SceneComponent.K2_GetComponentToWorld` (`GGJ_2025Character.FirstPersonCameraComponent` (`self.PlayerRef`)))))
  (:`Started`
    (if (`self.BuildMode ?`)
      (bind (_outhit _returnvalue) (`KismetSystemLibrary.LineTraceSingle` :`Start` _returnvalue_location :`End` (+ _returnvalue_location (* (`KismetMathLibrary.GetForwardVector` _returnvalue_rotation) (`self.DistanceToDrop`))) :`TraceChannel` "TraceTypeQuery1" :`DrawDebugType` "ForOneFrame"))
      (if _returnvalue
        (bind (_bblockinghit _binitialoverlap _time _distance _location _impactpoint _normal _impactnormal _physmat _hitactor) (`GameplayStatics.BreakHitResult` _outhit))
        (bind _asbp_parent_machines (cast `/Game/GGJ/Blueprint/Machines/BP_ParentMachines` _hitactor))
        (set `self.NewVar` (`SceneComponent.K2_GetComponentLocation` (`/Game/GGJ/Blueprint/Machines/BP_ParentMachines.Machine` _asbp_parent_machines)))
        (switch `/Game/GGJ/Blueprint/Machines/E_TypeBuild` (`/Game/GGJ/Blueprint/Machines/BP_ParentMachines.TypeBuild` _asbp_parent_machines)
          (:`NewEnumerator1`
            (bind _row_name (`/Game/GGJ/Blueprint/Machines/BP_ParentMachines.Row Name` _asbp_parent_machines))
            (bind _returnvalue_2 (`|GetDataTableRow` "/Game/GGJ/Blueprint/Machines/DT_Build.DT_Build" _row_name :!label _label_5)
              (:`then`
                (set `/Game/GGJ/Blueprint/FirstPerson/Blueprints/BP_FirstPersonCharacter.Gold` (+ (/ (`.Price_6_5A054677451A8E53069F469202B1236B` (break `/Game/GGJ/Blueprint/Machines/S_Build` _returnvalue_2)) 2) (`/Game/GGJ/Blueprint/FirstPerson/Blueprints/BP_FirstPersonCharacter.Gold` _playerref_2)) _playerref_2)
                (`/Game/GGJ/Blueprint/GI_CustomGameInstance.SaveGold` _asgi_custom_game_instance 0.0)
                (`/Game/GGJ/Blueprint/GI_CustomGameInstance.SaveBatRemove` _asgi_custom_game_instance (`Actor.GetTransform` _hitactor))
                (`Actor.K2_DestroyActor` _asbp_parent_machines))))
          (:`NewEnumerator2`
            (goto _label_5))
          (:`NewEnumerator3`
            (goto _label_5))
          (:`NewEnumerator4`
            (bind _asbp_spline (cast `/Game/GGJ/Blueprint/Machines/BP_Spline` _asbp_parent_machines))
            (bind _returnvalue_3 (`|GetDataTableRow` "/Game/GGJ/Blueprint/Machines/DT_Build.DT_Build" _row_name)
              (:`then`
                (set `/Game/GGJ/Blueprint/FirstPerson/Blueprints/BP_FirstPersonCharacter.Gold` (+ (/ (`.Price_6_5A054677451A8E53069F469202B1236B` (break `/Game/GGJ/Blueprint/Machines/S_Build` _returnvalue_3)) 2) (`/Game/GGJ/Blueprint/FirstPerson/Blueprints/BP_FirstPersonCharacter.Gold` _playerref)) _playerref)
                (`/Game/GGJ/Blueprint/GI_CustomGameInstance.SaveGold` _asgi_custom_game_instance 0.0)
                (`/Game/GGJ/Blueprint/GI_CustomGameInstance.SaveBatRemove` :`self` _asgi_custom_game_instance)
                (`/Game/GGJ/Blueprint/Machines/BP_Spline.DestroyEvent` _asbp_spline)))))
        (`GameplayStatics.PlaySound2D` "/Game/UI_SFX_Free_Pack/Cues/Purchase/coins_1_Cue.coins_1_Cue" 1.0 1.0 0.0 null null)
        (`NiagaraFunctionLibrary.SpawnSystemAtLocation` "/Game/GGJ/Mat/NS_Sell.NS_Sell" (`self.NewVar`))))))