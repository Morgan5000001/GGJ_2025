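; Holds a player's item inventory, loading it from the game instance's save by player ID and receiving bubbles through AddBubbleToInventory.
; Shared add and remove helpers return the updated inventory, with additions passed a maximum quantity.
; The open-inventory input toggles WBP_Inventory with that data, switching cursor and input mode.
; Debug keys add or remove random DT_Item entries; the Tick debug loop does nothing, its print left unconnected.
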(event Custom|AddBubbleToInventory
  (params (Item%20to%20add :type S%20Item%20Structure) (QuantityItem :type Integer))
  (bind _return_inventory (CallFunction|AddItemInventory Item%20to%20add QuantityItem (Variables|Default|GetInventory) (Variables|Default|GetQuantityMax)))
  (Variables|Default|SetInventory _return_inventory))

(event Custom|InitInventory
  (bind _asgi_custom_game_instance (Utilities|Casting|CastToGI_CustomGameInstance (Game|GetGameInstance)))
  (bind _saveref (Variables|/Game/GGJ/Blueprint/GI_CustomGameInstance.GI_CustomGameInstance_C|GetSaveRef _asgi_custom_game_instance)
    (:then
      (Variables|Default|SetInventory (.Value (Utilities|Map|Find (Variables|/Game/GGJ/Blueprint/BP_CustomSave.BP_CustomSave_C|GetInventory _saveref) (Variables|Default|GetID_Player)))))
    (:else)))

(event Input|EnhancedActionEvents|EnhancedInputActionIA_OpenInventory
  (params (ActionValue :type Boolean) (ElapsedSeconds :type Float%20%28double-precision%29) (TriggeredSeconds :type Float%20%28double-precision%29) (InputAction :type Input%20Action%20Object%20Reference :default "/Game/GGJ/Blueprint/FirstPerson/Input/Actions/IA_OpenInventory.IA_OpenInventory"))
  (bind _returnvalue (Game|GetPlayerController 0))
  (bind _returnvalue_2 (Game|GetPlayerController 0))
  (:Started
    (bind _inventorywidget (Variables|Default|GetInventoryWidget)
      (:then
        (Widget|RemovefromParent _inventorywidget)
        (Variables|Default|SetInventoryWidget 0)
        (Variables|/Script/Engine.PlayerController|SetbShowMouseCursor _returnvalue false)
        (Input|SetInputModeGameOnly _returnvalue true))
      (:else
        (bind _returnvalue_3 (UserInterface|CreateWidget "/Game/GGJ/Blueprint/Inventory/Widget/WBP_Inventory.WBP_Inventory_C" 0 (Variables|Default|GetInventory)))
        (bind _output_get (Variables|Default|SetInventoryWidget _returnvalue_3))
        (UserInterface|Viewport|AddtoViewport _output_get 0)
        (Variables|/Script/Engine.PlayerController|SetbShowMouseCursor _returnvalue_2 true)
        (Input|SetInputModeGameandUI _returnvalue_2 (Variables|Default|GetInventoryWidget) "DoNotLock" true true)))))

(event EventTick
  (params (DeltaSeconds :type Float%20%28single-precision%29))
  ;[1 1 1] Debug
  (for _array_element (Utilities|Struct|BreakS_Inventory (Variables|Default|GetInventory))
    _))

(event Input|KeyboardEvents|DebugKeyAdd
  (params (Key :type Key%20Structure :default "None") (ActionValue :type Input%20Action%20Value%20Structure))
  (:Pressed
    (bind _outrownames (DataTable|GetDataTableRowNames "/Game/GGJ/Blueprint/Inventory/DT_Item.DT_Item"))
    (bind _returnvalue (Utilities|GetDataTableRow "/Game/GGJ/Blueprint/Inventory/DT_Item.DT_Item" (.OutItem (Utilities|Array|Random _outrownames)))
      (:then
        (bind _return_inventory (CallFunction|AddItemInventory _returnvalue 7 (Variables|Default|GetInventory) (Variables|Default|GetQuantityMax)))
        (Variables|Default|SetInventory _return_inventory)))))

(event Input|KeyboardEvents|DebugKeySubtract
  (params (Key :type Key%20Structure :default "None") (ActionValue :type Input%20Action%20Value%20Structure))
  (:Pressed
    (bind _outrownames (DataTable|GetDataTableRowNames "/Game/GGJ/Blueprint/Inventory/DT_Item.DT_Item"))
    (bind _returnvalue (Utilities|GetDataTableRow "/Game/GGJ/Blueprint/Inventory/DT_Item.DT_Item" (.OutItem (Utilities|Array|Random _outrownames)))
      (:then
        (bind _return_inventory (CallFunction|RemoveItemInventory _returnvalue 1 (Variables|Default|GetInventory)))
        (Variables|Default|SetInventory _return_inventory)))))