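; BPC_Interact is a component that handles the player's interact input.
; On Interact, a sphere trace runs forward from the first-person camera, with persistent debug drawing.
; Outside build mode, the hit actor receives InteractMessage.
; In build mode with a specific build index selected, it receives InteractSplineMessage with the stored machine as parent, and unconnected results update that stored machine for linking.
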(event `EnhancedInput|/Game/FirstPerson/Input/Actions/IA_Interact`
  (params (ActionValue :type Boolean) (ElapsedSeconds :type "Float (double-precision)") (TriggeredSeconds :type "Float (double-precision)") (InputAction :type "InputAction Object Reference" :default "/Game/FirstPerson/Input/Actions/IA_Interact.IA_Interact"))
  (bind (_returnvalue_location _returnvalue_rotation) (`KismetMathLibrary.BreakTransform` (`SceneComponent.K2_GetComponentToWorld` (`GGJ_2025Character.FirstPersonCameraComponent` (`self.PlayerRef`)))))
  ;[1 0.786 0] Line trace t'es pas trop con
  (:`Started`
    (bind (_outhit _returnvalue) (`KismetSystemLibrary.SphereTraceSingle` :`Start` _returnvalue_location :`End` (+ _returnvalue_location (* (`KismetMathLibrary.GetForwardVector` _returnvalue_rotation) 300.0)) :`Radius` 50.0 :`TraceChannel` "TraceTypeQuery1" :`DrawDebugType` "Persistent"))
    ;[1 1 1] Branche d'arbre
    (if _returnvalue
      (if (not (`/Game/GGJ/Blueprint/BuildMode/BP_BuildComponent.BuildMode ?` (`/Game/FirstPerson/Blueprints/BP_FirstPersonCharacter.BP_BuildComponent` (`self.PlayerRef`))))
        (bind (_bblockinghit _binitialoverlap _time _distance _location _impactpoint _normal _impactnormal _physmat _hitactor) (`GameplayStatics.BreakHitResult` _outhit))
        (message `/Game/GGJ/Blueprint/Interact/BPI_Interact.Interact` _hitactor (`self.PlayerRef`))
        (elif (== (`/Game/GGJ/Blueprint/BuildMode/BP_BuildComponent.SelectIndex` (`/Game/FirstPerson/Blueprints/BP_FirstPersonCharacter.BP_BuildComponent` (`self.PlayerRef`))) 3)
          (bind (_machineshitted _isconnected) (message `/Game/GGJ/Blueprint/Interact/BPI_Interact.InteractSpline` _hitactor self (`self.Machines`)))
          (if (not _isconnected)
            (set `self.Machines` _machineshitted)))))))