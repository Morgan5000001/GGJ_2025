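; BP_BoomBox is an interactable boombox actor that plays and stops a sound in the world.
; Interact toggles on the IsOn flag, calling either RS_ActivateBoomBox or RS_StopIt.
; Activation spawns SC_Boombox at the actor's location and stores its reference, which stopping uses to silence it.
; Stopping also clears a timer handle that these graphs never set, and InteractSpline always reports no connection.
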(event `/Game/GGJ/Blueprint/Interact/BPI_Interact.Interact`
  (params (PlayerRef :type "/Game/GGJ/Blueprint/FirstPerson/Blueprints/BP_FirstPersonCharacter Object Reference"))
  ;[1 1 1] Interaction avec elle
  (if (`self.IsOn?`)
    (`self.RS_StopIt`)
    (else
      (`self.RS_ActivateBoomBox`))))

(event `RS_ActivateBoomBox`
  ;[1 1 1] Activaion du son de la boombox
  (bind _returnvalue (`GameplayStatics.SpawnSoundAtLocation` "/Game/GGJ/Import/Sound/SC_Boombox.SC_Boombox" (`self.K2_GetActorLocation`) (struct) 1.0 1.0 0.0 null null))
  (set `self.SoundRef` _returnvalue)
  (set `self.IsOn?` true))

(event `RS_StopIt`
  ;[1 1 1] Coupe le son de la boom box
  (set `self.IsOn?` false)
  (`AudioComponent.Stop` (`self.SoundRef`))
  (`KismetSystemLibrary.K2_ClearAndInvalidateTimerHandle` (`self.TimerHandle`)))

(fn `InteractSpline`
  (params (BP_BuildComponentRef :type "/Game/GGJ/Blueprint/BuildMode/BP_BuildComponent Object Reference") (ValidParent :type "/Game/GGJ/Blueprint/Machines/BP_ParentMachines Object Reference"))
  (returns (MachinesHitted :type "/Game/GGJ/Blueprint/Machines/BP_ParentMachines Object Reference") (IsConnected :type Boolean))
  (return null false))

(fn `UserConstructionScript`)