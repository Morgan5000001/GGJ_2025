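; Tutorial component that walks the player through five ordered steps: sink, tablet, selling, factory placement and collecting bubbles in the factory.
; On BeginPlay it creates WBP_Tutoriel with a reference to itself and adds it to the viewport.
; Each interaction event advances or removes the widget only when Steps matches its stage; Steps is not changed here.
; DestroyAll removes the widget and destroys the component.
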(event `self.ReceiveBeginPlay`
  (bind _returnvalue (`|CreateWidget` "/Game/Blueprints/Tutoriel/WBP_Tutoriel.WBP_Tutoriel_C" null self))
  (bind _output_get (set `self.WBP_TutoRef` _returnvalue))
  (`UserWidget.AddToViewport` _output_get 0))

(event `DestroyAll`
  (`Widget.RemoveFromParent` (`self.WBP_TutoRef`))
  (`self.K2_DestroyComponent`))

(event `/Game/Blueprints/Tutoriel/BPi_Tutoriel.InteractEvier`
  (params (EvierRef :type "/Game/GGJ/Blueprint/Machines/BP_Evier Object Reference"))
  (if (== (`self.Steps`) 1)
    (`/Game/Blueprints/Tutoriel/WBP_Tutoriel.AfterEvier` (`self.WBP_TutoRef`))))

(event `self.ReceiveTick`
  (params (DeltaSeconds :type "Float (single-precision)")))

(event `/Game/Blueprints/Tutoriel/BPi_Tutoriel.InteractTablette`
  (if (== (`self.Steps`) 2)
    (`/Game/Blueprints/Tutoriel/WBP_Tutoriel.AfterTablette` (`self.WBP_TutoRef`))))

(event `/Game/Blueprints/Tutoriel/BPi_Tutoriel.InteractSelling`
  (if (== (`self.Steps`) 3)
    (`/Game/Blueprints/Tutoriel/WBP_Tutoriel.AfterSelling` (`self.WBP_TutoRef`))))

(event `/Game/Blueprints/Tutoriel/BPi_Tutoriel.PlaceUsine`
  (if (== (`self.Steps`) 4)
    (`/Game/Blueprints/Tutoriel/WBP_Tutoriel.AfterPlace` (`self.WBP_TutoRef`))))

(event `/Game/Blueprints/Tutoriel/BPi_Tutoriel.GetBubblesInUsine`
  (if (== (`self.Steps`) 5)
    (`/Game/Blueprints/Tutoriel/WBP_Tutoriel.Remove` (`self.WBP_TutoRef`))))